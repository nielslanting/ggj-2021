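; Player controller that turns interact, directional and escape input into event dispatcher calls for other objects to handle.
; MoveForward and MoveRight axes become repeated direction presses, with a time-based cooldown lerped by deflection; once axis events fire, separate direction actions are ignored.
; Escape asks BP_GGJ_HUD to show its menu, otherwise broadcasts the press.
; Restart reloads maps with "Level" in their name, and a Debug action spawns another local player.
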(event `InputAction|Interact` :consume false
  (params (Key :type "Key Structure"))
  (:`Pressed`
    (`self.OnInteractPressed`))
  (:`Released`
    (`self.OnInteractReleased`)))

(event `InputAction|Down` :consume false
  (params (Key :type "Key Structure"))
  (:`Pressed`
    (if (not (`self.CanReceiveInputAxisMoveInstructions`))
      (`self.OnDownPressed`))))

(event `InputAction|Up` :consume false
  (params (Key :type "Key Structure"))
  (:`Pressed`
    (if (not (`self.CanReceiveInputAxisMoveInstructions`))
      (`self.OnUpPressed`))))

(event `InputAction|Left` :consume false
  (params (Key :type "Key Structure"))
  (:`Pressed`
    (if (not (`self.CanReceiveInputAxisMoveInstructions`))
      (`self.OnLeftPressed`))))

(event `InputAction|Right` :consume false
  (params (Key :type "Key Structure"))
  (:`Pressed`
    (if (not (`self.CanReceiveInputAxisMoveInstructions`))
      (`self.OnRightPressed`))))

(event `InputAxis|MoveForward` :consume false :overrideparent false
  (params (AxisValue :type "Float (single-precision)"))
  (set `self.CanReceiveInputAxisMoveInstructions` true)
  (if (> (`KismetMathLibrary.UtcNow`) (`self.ForwardThumbstickEnableDateTime`))
    (if (not (> AxisValue 0.5))
      (if (not (not (< AxisValue -0.05)))
        (`self.OnDownPressed`)
        (`self.FowardThumbstickCooldown` AxisValue))
      (else
        (`self.OnUpPressed`)
        (`self.FowardThumbstickCooldown` AxisValue)))
    (elif (== AxisValue 0.0)
      (set `self.ForwardThumbstickEnableDateTime` (`KismetMathLibrary.UtcNow`)))))

(event `InputAxis|MoveRight` :consume false :overrideparent false
  (params (AxisValue :type "Float (single-precision)"))
  (set `self.CanReceiveInputAxisMoveInstructions` true)
  (if (> (`KismetMathLibrary.UtcNow`) (`self.RightThumbstickEnableDateTime_0`))
    (if (not (> AxisValue 0.5))
      (if (not (not (< AxisValue -0.05)))
        (`self.OnLeftPressed`)
        (`self.RightThumbstickCooldown` AxisValue))
      (else
        (`self.OnRightPressed`)
        (`self.RightThumbstickCooldown` AxisValue)))
    (elif (== AxisValue 0.0)
      (set `self.RightThumbstickEnableDateTime_0` (`KismetMathLibrary.UtcNow`)))))

(event `FowardThumbstickCooldown`
  (params (AxisValue :type "Float (double-precision)"))
  (set `self.ForwardThumbstickEnableDateTime` (+ (`KismetMathLibrary.UtcNow`) (`KismetMathLibrary.MakeTimespan` 0 0 0 0 (`KismetMathLibrary.FTrunc` (`KismetMathLibrary.Lerp` (`self.MaxThumbsticTick`) (`self.MinThumbstickTick`) (`KismetMathLibrary.Abs` AxisValue)))))))

(event `RightThumbstickCooldown`
  (params (AxisValue :type "Float (double-precision)"))
  (set `self.RightThumbstickEnableDateTime_0` (+ (`KismetMathLibrary.UtcNow`) (`KismetMathLibrary.MakeTimespan` 0 0 0 0 (`KismetMathLibrary.FTrunc` (`KismetMathLibrary.Lerp` (`self.MaxThumbsticTick`) (`self.MinThumbstickTick`) (`KismetMathLibrary.Abs` AxisValue)))))))

(event `InputAction|Escape` :consume false
  (params (Key :type "Key Structure"))
  (:`Pressed`
    (`self.Escape`)))

(event `Escape`
  (bind _asbp_ggj_hud (cast `/Game/Blueprints/BP_GGJ_HUD` (`self.GetHUD`))
    (:`then`
      (bind _returnvalue (`/Game/Blueprints/BP_GGJ_HUD.CanShowEscapeMenu` _asbp_ggj_hud))
      (if _returnvalue
        (`/Game/Blueprints/BP_GGJ_HUD.ShowEscapeMenu` _asbp_ggj_hud)
        (else
          (`self.OnEscapePressed` :!label _label))))
    (:`CastFailed`
      (goto _label))))

(event `InputAction|Restart`
  (params (Key :type "Key Structure"))
  (:`Pressed`
    (`self.Restart`)))

(event `InputAction|SoftEscape`
  (params (Key :type "Key Structure"))
  (:`Pressed`
    (`self.OnSoftEscapePressed`)))

(event `Restart`
  (bind _returnvalue (`GameplayStatics.GetCurrentLevelName` true))
  (if (`KismetStringLibrary.Contains` _returnvalue "Level")
    (bind _returnvalue_2 (`GameplayStatics.GetCurrentLevelName` true))
    (`GameplayStatics.OpenLevel` (`KismetStringLibrary.Conv_StringToName` _returnvalue_2))))

(event `InputAction|Debug`
  (params (Key :type "Key Structure"))
  (:`Pressed`
    (`GameplayStatics.CreatePlayer` -1)))

(fn `UserConstructionScript`)