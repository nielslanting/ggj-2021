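; BP_Blockoutbox_Timer is a blockout box actor that periodically switches between solid and absent on a fixed looping timer.
; BeginPlay calls the parent, then starts a looping timer that fires ToggleBlock every few seconds.
; ToggleBlock inverts actor collision and flips both visibility and hidden-in-game on the root, propagating to child components.
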(event `self.ReceiveBeginPlay`
  (`parent.ReceiveBeginPlay`)
  (`KismetSystemLibrary.K2_SetTimer` null "ToggleBlock" 5.0 true))

(event `ToggleBlock`
  (`self.SetActorEnableCollision` self (not (`self.GetActorEnableCollision` self)))
  (`SceneComponent.SetVisibility` (`self.Root`) (not (`SceneComponent.IsVisible` (`self.Root`))) true)
  (`SceneComponent.SetHiddenInGame` (`self.Root`) (not (`SceneComponent.bHiddenInGame` (`self.Root`))) true))

(fn `UserConstructionScript`
  (`parent.UserConstructionScript`))