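; Blockout box that works as a one-shot trigger, toggling tagged response blocks in the level.
; While a Pawn overlaps its Box and it is untriggered, Tick bobs the actor slightly above its initial location as a pulse.
; TriggerBox, which nothing in this graph calls, stops the pulse and calls ToggleBlock on every BP_Blockoutbox_Response_Up matching its TriggerTags.
; Ending the overlap also resets the position.
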(event `self.ReceiveBeginPlay`
  (`parent.ReceiveBeginPlay`)
  (`SceneComponent.SetMobility` (`self.Root`) "Movable")
  (set `self.InitialLocation` (`self.K2_GetActorLocation`)))

(event `self.ReceiveTick`
  (params (DeltaSeconds :type "Float (single-precision)"))
  (`self.TickPulse` DeltaSeconds)
  (`parent.ReceiveTick` DeltaSeconds))

(event `TriggerBox`
  (if (not (`self.HasTriggered`))
    (set `self.HasTriggered` true)
    (`self.ResetPulse`)
    (for _array_element (`self.TriggerTags`)
      (bind _outactors (`GameplayStatics.GetAllActorsOfClassWithTag` "/Game/Blueprints/Actors/BP_Blockoutbox_Response_Up.BP_Blockoutbox_Response_Up_C" _array_element))
      (for _array_element_2 _outactors
        (`/Game/Blueprints/Actors/BP_Blockoutbox_Response_Up.ToggleBlock` _array_element_2)))))

(event `TickPulse`
  (params (DeltaSeconds :type "Float (double-precision)"))
  (bind (_initiallocation_x _initiallocation_y _initiallocation_z) (`KismetMathLibrary.BreakVector` (`self.InitialLocation`)))
  (if (`self.ShouldPulse`)
    (set `self.OffsetY` (+ (`self.OffsetY`) (* (select `bool` (`self.IsPulsingUp`) :`false` -30.0 :`true` 30.0 :!type "Float (single-precision)") DeltaSeconds)))
    (`self.K2_SetActorLocation` self (`KismetMathLibrary.MakeVector` _initiallocation_x _initiallocation_y (+ _initiallocation_z (`self.OffsetY`))) false true)
    (if (not (> (`self.OffsetY`) 10.0))
      (if (not (not (< (`self.OffsetY`) 0.0)))
        (set `self.IsPulsingUp` true))
      (else
        (set `self.IsPulsingUp` false)))))

(event `self.Box.OnComponentBeginOverlap`
  (params (OverlappedComponent :type "PrimitiveComponent Object Reference") (OtherActor :type "Actor Object Reference") (OtherComp :type "PrimitiveComponent Object Reference") (OtherBodyIndex :type Integer) (bFromSweep :type Boolean) (SweepResult :type "HitResult Structure (by ref)"))
  (cast `Pawn` OtherActor)
  (if (not (`self.HasTriggered`))
    (set `self.ShouldPulse` true)))

(event `self.Box.OnComponentEndOverlap`
  (params (OverlappedComponent :type "PrimitiveComponent Object Reference") (OtherActor :type "Actor Object Reference") (OtherComp :type "PrimitiveComponent Object Reference") (OtherBodyIndex :type Integer))
  (cast `Pawn` OtherActor)
  (`self.ResetPulse`))

(event `ResetPulse`
  (set `self.ShouldPulse` false)
  (`self.K2_SetActorLocation` (`self.InitialLocation`) false true))

(fn `UserConstructionScript`
  (`parent.UserConstructionScript`))