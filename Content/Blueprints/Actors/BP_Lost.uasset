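; BP_Lost is a goal-giver character actor that displays the items the current goal requires in an overhead widget.
; FinishGoal checks an owner's inventory component, then removes the items and completes the GameState component's goal, or plays an error sound if items are missing.
; On BeginPlay, goal changes and completion, it rebuilds the widget and swaps to one of six random skeletal meshes, masked by an oversized gunshot particle burst.
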(event `self.ReceiveBeginPlay`
  (bind _returnvalue (`GameplayStatics.GetGameState`))
  (bind _returnvalue_2 (`self.GetComponentByClass` _returnvalue "/Game/Blueprints/GameStateComponents/BP_GameState_Goal_Component.BP_GameState_Goal_Component_C"))
  (`self.SelectRandomSkeletalMesh`)
  (`self.SetupWidget`)
  (`/Engine/EditorBlueprintResources/StandardMacros.IsValid` _returnvalue
    (:`Is Valid`
      (`/Engine/EditorBlueprintResources/StandardMacros.IsValid` _returnvalue_2
        (:`Is Valid`
          (add `/Game/Blueprints/GameStateComponents/BP_GameState_Goal_Component.OnGoalChanged` _returnvalue_2 (delegate `OnGoalChanged_Event_0`)))))))

(event `OnGoalChanged_Event_0`
  (`self.SelectRandomSkeletalMesh`)
  (`self.SetupWidget`))

(fn `FinishGoal`
  (params (Owner :type "Actor Object Reference"))
  (locals (InventoryRef :type "/Game/Blueprints/ActorComponents/BP_Inventory_ActorComponent Object Reference") (GoalRef :type "/Game/Blueprints/GameStateComponents/BP_GameState_Goal_Component Object Reference"))
  (bind _returnvalue (`self.GetComponentByClass` Owner "/Game/Blueprints/ActorComponents/BP_Inventory_ActorComponent.BP_Inventory_ActorComponent_C"))
  (`/Engine/EditorBlueprintResources/StandardMacros.IsValid` _returnvalue
    (:`Is Valid`
      (set `local.InventoryRef` _returnvalue)
      (bind _output_get (set `local.GoalRef` (`self.GetComponentByClass` (`GameplayStatics.GetGameState`) "/Game/Blueprints/GameStateComponents/BP_GameState_Goal_Component.BP_GameState_Goal_Component_C")))
      (bind (_returnvalue_2 _isvalid) (`/Game/Blueprints/GameStateComponents/BP_GameState_Goal_Component.GetCurrentGoal` _output_get))
      (if _isvalid
        (bind _items (break `/Game/Blueprints/GameStateComponents/BPS_Goal` _returnvalue_2))
        (bind _returnvalue_3 (`/Game/Blueprints/ActorComponents/BP_Inventory_ActorComponent.ContainsItems` (`local.InventoryRef`) _items))
        (if _returnvalue_3
          (`/Game/Blueprints/ActorComponents/BP_Inventory_ActorComponent.RemoveItems` (`local.InventoryRef`) _items)
          (`/Game/Blueprints/GameStateComponents/BP_GameState_Goal_Component.FinishCurrentGoal` (`local.GoalRef`))
          (`self.SelectRandomSkeletalMesh`)
          (`self.SetupWidget`)
          (else
            (`GameplayStatics.PlaySound2D` "/Game/Sounds/FX/S_Goal_NotCorrect.S_Goal_NotCorrect" 1.0 1.0 0.0 null null)))))))

(fn `SelectRandomSkeletalMesh`
  (`SkinnedMeshComponent.SetSkinnedAssetAndUpdate` (`self.SkeletalMesh`) (select `int` (`KismetMathLibrary.RandomInteger` 6) :`0` "/Game/PolygonGangWarfare/Meshes/Characters/SK_Chr_Asian_Gangster_Male_01.SK_Chr_Asian_Gangster_Male_01" :`1` "/Game/PolygonGangWarfare/Meshes/Characters/SK_Chr_British_Gangster_Male_01.SK_Chr_British_Gangster_Male_01" :`2` "/Game/PolygonGangWarfare/Meshes/Characters/SK_Chr_Cook_Female_01.SK_Chr_Cook_Female_01" :`3` "/Game/PolygonGangWarfare/Meshes/Characters/SK_Chr_Cook_Male_01.SK_Chr_Cook_Male_01" :`4` "/Game/PolygonGangWarfare/Meshes/Characters/SK_Chr_DEA_Agent_Female_01.SK_Chr_DEA_Agent_Female_01" :`5` "/Game/PolygonGangWarfare/Meshes/Characters/SK_Chr_DEA_Agent_Male_01.SK_Chr_DEA_Agent_Male_01" :!type "SkeletalMesh Object Reference") true)
  (`GameplayStatics.SpawnEmitterAttached` "/Game/PolygonGangWarfare/FX/FX_Gunshot.FX_Gunshot" (`self.SkeletalMesh`) "None" (0.0 0.0 0.0) (struct) (15.0 15.0 15.0)))

(fn `SetupWidget`
  (bind _returnvalue (`self.GetComponentByClass` (`GameplayStatics.GetGameState`) "/Game/Blueprints/GameStateComponents/BP_GameState_Goal_Component.BP_GameState_Goal_Component_C"))
  (`/Engine/EditorBlueprintResources/StandardMacros.IsValid` _returnvalue
    (:`Is Valid`
      (bind (_returnvalue_2 _isvalid) (`/Game/Blueprints/GameStateComponents/BP_GameState_Goal_Component.GetCurrentGoal` _returnvalue))
      (if _isvalid
        (bind _returnvalue_3 (`|CreateWidget` "/Game/Blueprints/Widgets/Overhead/W_Overhead_Goal.W_Overhead_Goal_C" null (`.Items_7_738242704F3DF8F655EBE297948F0B21` (break `/Game/Blueprints/GameStateComponents/BPS_Goal` _returnvalue_2))))
        (`WidgetComponent.SetWidget` (`self.Widget`) _returnvalue_3)))))

(fn `UserConstructionScript`)