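; A moveable blockout box actor that travels back and forth along its spline indefinitely.
; On BeginPlay it makes its root movable and detaches the spline in world space so the path stays put while the box moves.
; A timeline scaled by Duration sets the root's position by distance along the spline, alternating forward and reverse.
; Characters that overlap the actor get a small upward launch.
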(event `self.ReceiveBeginPlay`
  (`parent.ReceiveBeginPlay`)
  (`TimelineComponent.SetPlayRate` (`self.ForwardTimeline`) (/ 1.0 (`self.Duration`)))
  (`SceneComponent.SetMobility` (`self.Root`) "Movable")
  (set `self.InitialLocation` (`SceneComponent.K2_GetComponentLocation` (`self.Root`)))
  (`SceneComponent.K2_DetachFromComponent` (`self.Spline`) "KeepWorld" "KeepWorld" "KeepWorld" true)
  (bind (_direction _traveltrack) (`Timeline|ForwardTimeline` :!via `PlayFromStart` :!label _label)
    (:`Update`
      (`SceneComponent.K2_SetWorldLocation` (`self.Root`) (`SplineComponent.GetLocationAtDistanceAlongSpline` (`self.Spline`) (* (`SplineComponent.GetSplineLength` (`self.Spline`)) _traveltrack) "World") false false))
    (:`Finished`
      (if (`|EnumEquality` _direction "Forward")
        (goto _label :!via `Reverse`)
        (else
          (goto _label :!via `PlayFromStart`))))))

(event `self.ReceiveActorBeginOverlap`
  (params (OtherActor :type "Actor Object Reference"))
  (bind _ascharacter (cast `Character` OtherActor))
  (`Character.LaunchCharacter` _ascharacter (0.0 0.0 10.0) false false))

(fn `UserConstructionScript`
  (`parent.UserConstructionScript`))