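; Blockout box actor that starts flattened and pops up to full height after being touched.
; BeginPlay saves the Root's scale and squashes its Z to a tenth.
; The first overlap on Box waits a second, restores the scale, plays a particle effect and sound, then sets HasPopped to prevent repeats.
; A separate ToggleBlock event flips collision, visibility and hidden-in-game state.
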(event `self.ReceiveBeginPlay`
  (bind (_initialscale_x _initialscale_y _initialscale_z) (`KismetMathLibrary.BreakVector` (`self.InitialScale`)))
  (`parent.ReceiveBeginPlay`)
  (set `self.InitialScale` (`SceneComponent.K2_GetComponentScale` (`self.Root`)))
  (`SceneComponent.SetWorldScale3D` (`self.Root`) (`KismetMathLibrary.MakeVector` _initialscale_x _initialscale_y (/ _initialscale_z 10.0))))

(event `ToggleBlock`
  (`self.SetActorEnableCollision` self (not (`self.GetActorEnableCollision` self)))
  (`SceneComponent.SetVisibility` (`self.Root`) (not (`SceneComponent.IsVisible` (`self.Root`))) true)
  (`SceneComponent.SetHiddenInGame` (`self.Root`) (not (`SceneComponent.bHiddenInGame` (`self.Root`))) true))

(event `self.Box.OnComponentBeginOverlap`
  (params (OverlappedComponent :type "PrimitiveComponent Object Reference") (OtherActor :type "Actor Object Reference") (OtherComp :type "PrimitiveComponent Object Reference") (OtherBodyIndex :type Integer) (bFromSweep :type Boolean) (SweepResult :type "HitResult Structure (by ref)"))
  (if (not (`self.HasPopped`))
    (`KismetSystemLibrary.Delay` 1.0)
    (`SceneComponent.SetWorldScale3D` (`self.Root`) (`self.InitialScale`))
    (`GameplayStatics.SpawnEmitterAttached` "/Game/PolygonGangWarfare/FX/FX_Gunshot.FX_Gunshot" (`self.Root`) "None" (0.0 0.0 0.0) (struct) (15.0 15.0 15.0))
    (`GameplayStatics.PlaySound2D` "/Game/Sounds/FX/S_ResponseBox_Popup.S_ResponseBox_Popup" 1.0 1.0 0.0 null null)
    (set `self.HasPopped` true)))

(fn `UserConstructionScript`
  (`parent.UserConstructionScript`))