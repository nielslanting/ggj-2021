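; Pushable blockout box that slides along the X or Y axis when a Character pushes against one of its sides.
; Four side trigger boxes start a delay on overlap, then push the box the opposite way if that side's flag is set.
; A short Visibility trace blocks obstructed moves; otherwise a DoOnce-guarded timeline slides the root up to 50 units with a sound.
; Only the left side's end overlap clears its own flag.
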(event `self.ReceiveBeginPlay`
  (`parent.ReceiveBeginPlay`)
  (`SceneComponent.SetMobility` (`self.Root`) "Movable"))

(event `self.LeftBox.OnComponentBeginOverlap`
  (params (OverlappedComponent :type "PrimitiveComponent Object Reference") (OtherActor :type "Actor Object Reference") (OtherComp :type "PrimitiveComponent Object Reference") (OtherBodyIndex :type Integer) (bFromSweep :type Boolean) (SweepResult :type "HitResult Structure (by ref)"))
  (cast `Character` OtherActor)
  (set `self.IsPushingLeft` true)
  (`KismetSystemLibrary.Delay` (`self.Delay`))
  (if (`self.IsPushingLeft`)
    (`self.PushRight`)))

(event `self.LeftBox.OnComponentEndOverlap`
  (params (OverlappedComponent :type "PrimitiveComponent Object Reference") (OtherActor :type "Actor Object Reference") (OtherComp :type "PrimitiveComponent Object Reference") (OtherBodyIndex :type Integer))
  (cast `Character` OtherActor)
  (set `self.IsPushingLeft` false))

(event `self.RightBox.OnComponentBeginOverlap`
  (params (OverlappedComponent :type "PrimitiveComponent Object Reference") (OtherActor :type "Actor Object Reference") (OtherComp :type "PrimitiveComponent Object Reference") (OtherBodyIndex :type Integer) (bFromSweep :type Boolean) (SweepResult :type "HitResult Structure (by ref)"))
  (cast `Character` OtherActor)
  (set `self.IsPushingRight` true)
  (`KismetSystemLibrary.Delay` (`self.Delay`))
  (if (`self.IsPushingRight`)
    (`self.PushLeft`)))

(event `self.RightBox.OnComponentEndOverlap`
  (params (OverlappedComponent :type "PrimitiveComponent Object Reference") (OtherActor :type "Actor Object Reference") (OtherComp :type "PrimitiveComponent Object Reference") (OtherBodyIndex :type Integer))
  (cast `Character` OtherActor)
  (set `self.IsPushingLeft` false))

(event `self.TopBox.OnComponentBeginOverlap`
  (params (OverlappedComponent :type "PrimitiveComponent Object Reference") (OtherActor :type "Actor Object Reference") (OtherComp :type "PrimitiveComponent Object Reference") (OtherBodyIndex :type Integer) (bFromSweep :type Boolean) (SweepResult :type "HitResult Structure (by ref)"))
  (cast `Character` OtherActor)
  (set `self.IsPushingTop` true)
  (`KismetSystemLibrary.Delay` (`self.Delay`))
  (if (`self.IsPushingTop`)
    (`self.PushBottom`)))

(event `self.TopBox.OnComponentEndOverlap`
  (params (OverlappedComponent :type "PrimitiveComponent Object Reference") (OtherActor :type "Actor Object Reference") (OtherComp :type "PrimitiveComponent Object Reference") (OtherBodyIndex :type Integer))
  (cast `Character` OtherActor)
  (set `self.IsPushingTop` true))

(event `self.BottomBox.OnComponentBeginOverlap`
  (params (OverlappedComponent :type "PrimitiveComponent Object Reference") (OtherActor :type "Actor Object Reference") (OtherComp :type "PrimitiveComponent Object Reference") (OtherBodyIndex :type Integer) (bFromSweep :type Boolean) (SweepResult :type "HitResult Structure (by ref)"))
  (cast `Character` OtherActor)
  (set `self.IsPusingBottom` true)
  (`KismetSystemLibrary.Delay` (`self.Delay`))
  (if (`self.IsPusingBottom`)
    (`self.PushTop`)))

(event `self.BottomBox.OnComponentEndOverlap`
  (params (OverlappedComponent :type "PrimitiveComponent Object Reference") (OtherActor :type "Actor Object Reference") (OtherComp :type "PrimitiveComponent Object Reference") (OtherBodyIndex :type Integer))
  (cast `Character` OtherComp)
  (set `self.IsPusingBottom` true))

(event `PushRight`
  (bind (_beforelocation_x _beforelocation_y _beforelocation_z) (`KismetMathLibrary.BreakVector` (`self.BeforeLocation`)))
  (bind _returnvalue (`SceneComponent.K2_GetComponentLocation` (`self.RightBox`)))
  (bind (_outhit _returnvalue_2) (`KismetSystemLibrary.LineTraceSingle` _returnvalue (+ _returnvalue (0.0 24.0 0.0)) "TraceTypeQuery1"))
  (if (not _returnvalue_2)
    (`/Engine/EditorBlueprintResources/StandardMacros.DoOnce` false :!label _label
      (:`Completed`
        (set `self.BeforeLocation` (`SceneComponent.RelativeLocation` (`self.Root`)))
        (`GameplayStatics.PlaySound2D` "/Game/Sounds/FX/S_SlotChange.S_SlotChange" 1.0 1.0 0.0 null null)
        (bind (_direction _pushtrack) (`Timeline|Push` :!via `PlayFromStart`)
          (:`Update`
            (`SceneComponent.K2_SetRelativeLocation` (`self.Root`) (`KismetMathLibrary.MakeVector` _beforelocation_x (+ (* _pushtrack 50.0) _beforelocation_y) _beforelocation_z) false true))
          (:`Finished`
            (goto _label :!via `Reset`)))))))

(event `PushLeft`
  (bind (_beforelocation_x _beforelocation_y _beforelocation_z) (`KismetMathLibrary.BreakVector` (`self.BeforeLocation`)))
  (bind _returnvalue (`SceneComponent.K2_GetComponentLocation` (`self.LeftBox`)))
  (bind (_outhit _returnvalue_2) (`KismetSystemLibrary.LineTraceSingle` _returnvalue (+ _returnvalue (0.0 -24.0 0.0)) "TraceTypeQuery1"))
  (if (not _returnvalue_2)
    (`/Engine/EditorBlueprintResources/StandardMacros.DoOnce` false :!label _label_2
      (:`Completed`
        (set `self.BeforeLocation` (`SceneComponent.RelativeLocation` (`self.Root`)))
        (`GameplayStatics.PlaySound2D` "/Game/Sounds/FX/S_SlotChange.S_SlotChange" 1.0 1.0 0.0 null null)
        (bind (_direction _pushtrack) (`Timeline|Timeline_0` :!via `PlayFromStart`)
          (:`Update`
            (`SceneComponent.K2_SetRelativeLocation` (`self.Root`) (`KismetMathLibrary.MakeVector` _beforelocation_x (+ (* _pushtrack -50.0) _beforelocation_y) _beforelocation_z) false true))
          (:`Finished`
            (goto _label_2 :!via `Reset`)))))))

(event `PushBottom`
  (bind (_beforelocation_x _beforelocation_y _beforelocation_z) (`KismetMathLibrary.BreakVector` (`self.BeforeLocation`)))
  (bind _returnvalue (`SceneComponent.K2_GetComponentLocation` (`self.BottomBox`)))
  (bind (_outhit _returnvalue_2) (`KismetSystemLibrary.LineTraceSingle` _returnvalue (+ _returnvalue (-24.0 0.0 0.0)) "TraceTypeQuery1"))
  (if (not _returnvalue_2)
    (`/Engine/EditorBlueprintResources/StandardMacros.DoOnce` false :!label _label_3
      (:`Completed`
        (set `self.BeforeLocation` (`SceneComponent.RelativeLocation` (`self.Root`)))
        (`GameplayStatics.PlaySound2D` "/Game/Sounds/FX/S_SlotChange.S_SlotChange" 1.0 1.0 0.0 null null)
        (bind (_direction _pushtrack) (`Timeline|Timeline_1`)
          (:`Update`
            (`SceneComponent.K2_SetRelativeLocation` (`self.Root`) (`KismetMathLibrary.MakeVector` (+ (* _pushtrack -50.0) _beforelocation_x) _beforelocation_y _beforelocation_z) false true))
          (:`Finished`
            (goto _label_3 :!via `Reset`)))))))

(event `PushTop`
  (bind (_beforelocation_x _beforelocation_y _beforelocation_z) (`KismetMathLibrary.BreakVector` (`self.BeforeLocation`)))
  (bind _returnvalue (`SceneComponent.K2_GetComponentLocation` (`self.TopBox`)))
  (bind (_outhit _returnvalue_2) (`KismetSystemLibrary.LineTraceSingle` _returnvalue (+ _returnvalue (24.0 0.0 0.0)) "TraceTypeQuery1"))
  (if (not _returnvalue_2)
    (`/Engine/EditorBlueprintResources/StandardMacros.DoOnce` false :!label _label_4
      (:`Completed`
        (set `self.BeforeLocation` (`SceneComponent.RelativeLocation` (`self.Root`)))
        (`GameplayStatics.PlaySound2D` "/Game/Sounds/FX/S_SlotChange.S_SlotChange" 1.0 1.0 0.0 null null)
        (bind (_direction _pushtrack) (`Timeline|Timeline_2` :!via `PlayFromStart`)
          (:`Update`
            (`SceneComponent.K2_SetRelativeLocation` (`self.Root`) (`KismetMathLibrary.MakeVector` (+ (* _pushtrack 50.0) _beforelocation_x) _beforelocation_y _beforelocation_z) false true))
          (:`Finished`
            (goto _label_4 :!via `Reset`)))))))

(fn `UserConstructionScript`
  (`parent.UserConstructionScript`))