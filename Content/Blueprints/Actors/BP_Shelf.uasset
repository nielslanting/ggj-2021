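; BP_Shelf is a shelf actor that stores items up to a capacity and pulses in size while a pawn is in range.
; On BeginPlay it fills its Items array from StartItems data table row references.
; It exposes store, retrieve-by-index, list and space-check calls, though storing does not itself enforce the limit.
; Box overlaps toggle a Tick-driven root-scale oscillation, reset when a pawn leaves.
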(event `self.ReceiveBeginPlay`
  (`self.SetupStartItems`))

(event `self.ReceiveTick`
  (params (DeltaSeconds :type "Float (single-precision)"))
  (`self.TickPulse` DeltaSeconds))

(event `/Game/Blueprints/Interfaces/BPI_StorageUnit.StoreItem`
  (params (Item :type "/Game/Data/BPS_Item Structure"))
  (`KismetArrayLibrary.Array_Add` (`self.Items`) Item))

(event `SetupStartItems`
  (for _array_element (`self.StartItems`)
    (bind _returnvalue (`|GetDataTableRow` (break `DataTableRowHandle` _array_element) (`.RowName` (break `DataTableRowHandle` _array_element)))
      (:`then`
        (`KismetArrayLibrary.Array_Add` (`self.Items`) _returnvalue)))))

(event `self.Box.OnComponentBeginOverlap`
  (params (OverlappedComponent :type "PrimitiveComponent Object Reference") (OtherActor :type "Actor Object Reference") (OtherComp :type "PrimitiveComponent Object Reference") (OtherBodyIndex :type Integer) (bFromSweep :type Boolean) (SweepResult :type "HitResult Structure (by ref)"))
  (cast `Pawn` OtherActor)
  (set `self.ShouldPulse` true))

(event `self.Box.OnComponentEndOverlap`
  (params (OverlappedComponent :type "PrimitiveComponent Object Reference") (OtherActor :type "Actor Object Reference") (OtherComp :type "PrimitiveComponent Object Reference") (OtherBodyIndex :type Integer))
  (cast `Pawn` OtherActor)
  (set `self.ShouldPulse` false)
  (set `self.Scale` 1.0)
  (`SceneComponent.SetRelativeScale3D` (`self.DefaultSceneRoot`) (`KismetMathLibrary.Conv_DoubleToVector` (`self.Scale`))))

(event `TickPulse`
  (params (DeltaSeconds :type "Float (double-precision)"))
  (if (`self.ShouldPulse`)
    (bind _output_get (set `self.Scale` (+ (`self.Scale`) (* (select `bool` (`self.IsGrowing`) :`false` -0.1 :`true` 0.1 :!type "Float (single-precision)") DeltaSeconds))))
    (`SceneComponent.SetRelativeScale3D` (`self.DefaultSceneRoot`) (`KismetMathLibrary.Conv_DoubleToVector` _output_get))
    (if (not (> (`self.Scale`) 1.01))
      (if (not (not (< (`self.Scale`) 0.99)))
        (set `self.IsGrowing` true))
      (else
        (set `self.IsGrowing` false)))))

(fn `GetItems`
  (returns (ReturnValue :type "Array of /Game/Data/BPS_Item Structure"))
  (return (`self.Items`)))

(fn `HasSpace`
  (returns (ReturnValue :type Boolean))
  (return (< (`KismetArrayLibrary.Array_Length` (`self.Items`)) (`self.MaxItems`))))

(fn `RetrieveItem`
  (params (index :type Integer))
  (returns (ReturnValue :type "/Game/Data/BPS_Item Structure"))
  (locals (Result :type "/Game/Data/BPS_Item Structure"))
  (set `local.Result` (`|GetArrayItem` (`self.Items`) index))
  (`KismetArrayLibrary.Array_Remove` (`self.Items`) index)
  (return (`local.Result`)))

(fn `UserConstructionScript`)