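; Blockout box response actor that starts flattened and pops up to full height when its ToggleBlock event is called.
; BeginPlay caches the root's world scale, then squashes Z to a tenth of it.
; ToggleBlock restores the cached scale with an attached gunshot particle effect and a 2D popup sound; despite the name, it never lowers the block again.
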(event `self.ReceiveBeginPlay`
  (bind (_initialscale_x _initialscale_y _initialscale_z) (`KismetMathLibrary.BreakVector` (`self.InitialScale`)))
  (`parent.ReceiveBeginPlay`)
  (set `self.InitialScale` (`SceneComponent.K2_GetComponentScale` (`self.Root`)))
  (`SceneComponent.SetWorldScale3D` (`self.Root`) (`KismetMathLibrary.MakeVector` _initialscale_x _initialscale_y (* _initialscale_z 0.1))))

(event `ToggleBlock`
  (bind (_initialscale_x _initialscale_y _initialscale_z) (`KismetMathLibrary.BreakVector` (`self.InitialScale`)))
  (`SceneComponent.SetWorldScale3D` (`self.Root`) (`KismetMathLibrary.MakeVector` _initialscale_x _initialscale_y _initialscale_z))
  (`GameplayStatics.SpawnEmitterAttached` "/Game/PolygonGangWarfare/FX/FX_Gunshot.FX_Gunshot" (`self.Root`) "None" (0.0 0.0 0.0) (struct) (15.0 15.0 15.0))
  (`GameplayStatics.PlaySound2D` "/Game/Sounds/FX/S_ResponseBox_Popup.S_ResponseBox_Popup" 1.0 1.0 0.0 null null))

(fn `UserConstructionScript`
  (`parent.UserConstructionScript`))