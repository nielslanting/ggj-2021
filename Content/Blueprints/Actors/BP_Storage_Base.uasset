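; BP_Storage_Base is a storage actor that holds items up to MaxItems and displays them on four slot static meshes.
; Start items load from data table rows, and each mesh is placed at its slot's cached location plus the item's transform.
; StoreItem appends and displays an item, while RetrieveItem removes one and rebuilds the slots.
; While a pawn overlaps AnimationBox, Tick gently pulses the root's scale, resetting it on exit.
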(event `self.ReceiveBeginPlay`
  (`self.ResetStaticMeshes`)
  (`self.SetupInitialTransforms`)
  (`self.SetupStartItems`))

(event `self.ReceiveTick`
  (params (DeltaSeconds :type "Float (single-precision)"))
  (`self.TickPulse` DeltaSeconds))

(event `ResetStaticMeshes`
  (for _index (range (`self.MaxItems`))
    (bind _returnvalue (`self.GetStaticmeshRefBySlot` _index))
    (`StaticMeshComponent.SetStaticMesh` _returnvalue null)))

(event `SetupInitialTransforms`
  (for _index (range (`self.MaxItems`))
    (bind _returnvalue (`self.GetStaticmeshRefBySlot` _index))
    (`KismetArrayLibrary.Array_Add` (`self.InitialTransforms`) (`SceneComponent.GetRelativeTransform` _returnvalue))))

(event `/Game/Blueprints/Interfaces/BPI_StorageUnit.StoreItem`
  (params (Item :type "/Game/Data/BPS_Item Structure"))
  (`KismetArrayLibrary.Array_Add` (`self.Items`) Item)
  (`self.SetupItemStaticMesh` (`KismetArrayLibrary.Array_LastIndex` (`self.Items`))))

(event `SetupStartItems`
  (for _array_element (`self.StartItems`)
    (bind _returnvalue (`|GetDataTableRow` (break `DataTableRowHandle` _array_element) (`.RowName` (break `DataTableRowHandle` _array_element)))
      (:`then`
        (`KismetArrayLibrary.Array_Add` (`self.Items`) _returnvalue)
        (`self.SetupItemStaticMesh` (`KismetArrayLibrary.Array_LastIndex` (`self.Items`)))))))

(event `SetupItemStaticMesh`
  (params (Slot :type Integer))
  (bind _output_location (`KismetMathLibrary.BreakTransform` (`|GetArrayItem` (`self.InitialTransforms`) Slot)))
  (bind (_staticmesh _name _preview _transform) (break `/Game/Data/BPS_Item` (`|GetArrayItem` (`self.Items`) Slot)))
  (bind _returnvalue (`self.GetStaticmeshRefBySlot` Slot))
  (`StaticMeshComponent.SetStaticMesh` _returnvalue _staticmesh)
  (`SceneComponent.K2_SetRelativeTransform` _returnvalue (`KismetMathLibrary.MakeTransform` (+ _output_location (.location _transform)) (.rotation _transform) (.scale _transform)) false true))

(event `self.AnimationBox.OnComponentBeginOverlap`
  (params (OverlappedComponent :type "PrimitiveComponent Object Reference") (OtherActor :type "Actor Object Reference") (OtherComp :type "PrimitiveComponent Object Reference") (OtherBodyIndex :type Integer) (bFromSweep :type Boolean) (SweepResult :type "HitResult Structure (by ref)"))
  (cast `Pawn` OtherActor)
  (set `self.ShouldPulse` true))

(event `self.AnimationBox.OnComponentEndOverlap`
  (params (OverlappedComponent :type "PrimitiveComponent Object Reference") (OtherActor :type "Actor Object Reference") (OtherComp :type "PrimitiveComponent Object Reference") (OtherBodyIndex :type Integer))
  (cast `Pawn` OtherActor)
  (set `self.ShouldPulse` false)
  (set `self.Scale` 1.0)
  (`SceneComponent.SetRelativeScale3D` (`self.DefaultSceneRoot`) (`KismetMathLibrary.Conv_DoubleToVector` (`self.Scale`))))

(event `TickPulse`
  (params (DeltaSeconds :type "Float (double-precision)"))
  (if (`self.ShouldPulse`)
    (bind _output_get (set `self.Scale` (+ (`self.Scale`) (* (select `bool` (`self.IsGrowing`) :`false` -0.1 :`true` 0.1 :!type "Float (single-precision)") DeltaSeconds))))
    (`SceneComponent.SetRelativeScale3D` (`self.DefaultSceneRoot`) (`KismetMathLibrary.Conv_DoubleToVector` _output_get))
    (if (not (> (`self.Scale`) 1.01))
      (if (not (not (< (`self.Scale`) 0.99)))
        (set `self.IsGrowing` true))
      (else
        (set `self.IsGrowing` false)))))

(fn `GetItems`
  (returns (ReturnValue :type "Array of /Game/Data/BPS_Item Structure"))
  (return (`self.Items`)))

(fn `GetStaticmeshRefBySlot`
  (params (Slot :type Integer))
  (returns (ReturnValue :type "StaticMeshComponent Object Reference"))
  (switch `int` Slot
    (:`Default`
      (return null))
    (:`0`
      (return (`self.Slot1`)))
    (:`1`
      (return (`self.Slot2`)))
    (:`2`
      (return (`self.Slot3`)))
    (:`3`
      (return (`self.Slot4`)))))

(fn `HasSpace`
  (returns (ReturnValue :type Boolean))
  (return (< (`KismetArrayLibrary.Array_Length` (`self.Items`)) (`self.MaxItems`))))

(fn `RetrieveItem`
  (params (index :type Integer))
  (returns (ReturnValue :type "/Game/Data/BPS_Item Structure"))
  (locals (Result :type "/Game/Data/BPS_Item Structure"))
  (set `local.Result` (`|GetArrayItem` (`self.Items`) index))
  (`KismetArrayLibrary.Array_Remove` (`self.Items`) index)
  (`self.ResetStaticMeshes`)
  (for (_ _array_index) (`self.Items`)
    (`self.SetupItemStaticMesh` _array_index))
  (return (`local.Result`)))

(fn `UserConstructionScript`)