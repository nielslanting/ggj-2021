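; BP_GGJ_GameState is a game state Blueprint that tracks score and failures from goal outcomes.
; On BeginPlay it binds to the goal component's finished and failed events.
; A finished goal increments the score component's score, while a failed goal increments its failure count, keeping goal logic and scoring in separate components.
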(event `self.ReceiveBeginPlay`
  (`self.SetupScoreGoalBinding`))

(event `SetupScoreGoalBinding`
  (add `/Game/Blueprints/GameStateComponents/BP_GameState_Goal_Component.OnGoalFinished` (`self.BP_GameState_Goal_Component`) (delegate `CustomEvent_0`))
  (add `/Game/Blueprints/GameStateComponents/BP_GameState_Goal_Component.OnGoalFailed` (`self.BP_GameState_Goal_Component`) (delegate `OnGoalFailed_Event_0`)))

(event `CustomEvent_0`
  (params (Goal :type "/Game/Blueprints/GameStateComponents/BPS_Goal Structure"))
  (`/Game/Blueprints/GameStateComponents/BP_GameState_Score_Component.IncreaseScore` (`self.BP_GameState_Score_Component`)))

(event `OnGoalFailed_Event_0`
  (`/Game/Blueprints/GameStateComponents/BP_GameState_Score_Component.IncreaseFailed` (`self.BP_GameState_Score_Component`)))

(fn `BP_GGJ_GameState_AutoGenFunc`
  (params (Goal :type "/Game/Blueprints/GameStateComponents/BPS_Goal Structure")))

(fn `UserConstructionScript`)