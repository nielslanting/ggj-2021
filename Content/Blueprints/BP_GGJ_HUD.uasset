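; HUD Blueprint for a game jam game that creates and manages the player's UI widgets.
; On BeginPlay it adds inventory, goals and current-level widgets, plus touch buttons on Android.
; Events show level completed or failed screens, a storage interaction panel and an escape menu that pauses via zero time dilation.
; Both closable panels disable pawn input until closed, and CanShowEscapeMenu reports whether neither is open.
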(event `self.ReceiveBeginPlay`
  (`self.SetupInventoryWidget`)
  (`self.SetupGoalWidget`)
  (`self.SetupCurrentLevelWidget`)
  (`self.SetupAndroid`))

(event `SetupInventoryWidget`
  (bind _returnvalue (`|CreateWidget` "/Game/Blueprints/Widgets/Inventory/W_Inventory.W_Inventory_C" (`self.GetOwningPlayerController`)))
  (bind _output_get (set `self.InventoryRef` _returnvalue))
  (`UserWidget.AddToPlayerScreen` _output_get -40))

(event `SetupGoalWidget`
  (bind _returnvalue (`|CreateWidget` "/Game/Blueprints/Widgets/Goals/W_Goals.W_Goals_C" (`self.GetOwningPlayerController`)))
  (bind _output_get (set `self.GoalsRef` _returnvalue))
  (`UserWidget.AddToPlayerScreen` _output_get 10))

(event `/Game/Blueprints/Interfaces/BPI_HUD_ShowLevelCompleteWidget.ShowLevelCompleteWidget`
  (params (CurrentLevel :type String) (CompletedIn :type Text) (NextLevelName :type Name))
  (bind _returnvalue (`|CreateWidget` "/Game/Blueprints/Widgets/W_LevelCompleted.W_LevelCompleted_C" (`self.GetOwningPlayerController`) NextLevelName))
  (`UserWidget.AddToViewport` _returnvalue 0)
  (`WidgetBlueprintLibrary.SetInputMode_GameAndUIEx` (`self.GetOwningPlayerController`) _returnvalue))

(event `/Game/Blueprints/Interfaces/BPI_HUD_ShowInteractWidget.ShowInteractWidget`
  (params (Storage :type "/Game/Blueprints/Interfaces/BPI_StorageUnit Interface"))
  (bind _interactref (`self.InteractRef`))
  (`/Engine/EditorBlueprintResources/StandardMacros.IsValid` _interactref
    (:`Is Valid`
      (if (not (`Widget.IsVisible` _interactref))
        (bind _returnvalue (`|CreateWidget` "/Game/Blueprints/Widgets/Interact/W_Interact.W_Interact_C" (`self.GetOwningPlayerController`) Storage :!label _label))
        (bind _output_get (set `self.InteractRef` _returnvalue))
        (`UserWidget.AddToPlayerScreen` _output_get -20)
        (add `/Game/Blueprints/Widgets/Interact/W_Interact.OnClose` _output_get (delegate `OnClose_Event_0`))
        (`WidgetBlueprintLibrary.SetInputMode_GameAndUIEx` (`self.GetOwningPlayerController`) _output_get)
        (`self.DisableInput` (`Controller.K2_GetPawn` (`self.GetOwningPlayerController`)) (`self.GetOwningPlayerController`))))
    (:`Is Not Valid`
      (goto _label))))

(event `OnClose_Event_0`
  (`/Engine/EditorBlueprintResources/StandardMacros.IsValid` (`self.InteractRef`)
    (:`Is Valid`
      (`Widget.RemoveFromParent` (`self.InteractRef`))
      (`KismetSystemLibrary.CollectGarbage`)
      (set `self.InteractRef` null)
      (`self.EnableInput` (`Controller.K2_GetPawn` (`self.GetOwningPlayerController`)) (`self.GetOwningPlayerController`)))))

(event `/Game/Blueprints/Interfaces/BPI_HUD_ShowLevelCompleteWidget.ShowLevelFailedWidget`
  (bind _returnvalue (`|CreateWidget` "/Game/Blueprints/Widgets/W_LevelFailed.W_LevelFailed_C" (`self.GetOwningPlayerController`)))
  (`UserWidget.AddToViewport` _returnvalue 0)
  (`WidgetBlueprintLibrary.SetInputMode_GameAndUIEx` (`self.GetOwningPlayerController`) _returnvalue))

(event `ShowEscapeMenu`
  (bind _returnvalue (`self.GetOwningPlayerController`))
  (`/Engine/EditorBlueprintResources/StandardMacros.IsValid` (`self.EscapeMenuRef`)
    (:`Is Not Valid`
      (bind _returnvalue_2 (`|CreateWidget` "/Game/Blueprints/Widgets/EscapeMenu/W_EscapeMenu.W_EscapeMenu_C" (`self.GetOwningPlayerController`)))
      (bind _output_get (set `self.EscapeMenuRef` _returnvalue_2))
      (add `/Game/Blueprints/Widgets/EscapeMenu/W_EscapeMenu.OnClose` _output_get (delegate `OnClose_Event_1`))
      (`UserWidget.AddToPlayerScreen` (`self.EscapeMenuRef`) -20)
      (`GameplayStatics.SetGlobalTimeDilation` 0.0)
      (`self.DisableInput` (`Controller.K2_GetPawn` _returnvalue) _returnvalue))))

(event `OnClose_Event_1`
  (bind _returnvalue (`self.GetOwningPlayerController`))
  (`Widget.RemoveFromParent` (`self.EscapeMenuRef`))
  (`KismetSystemLibrary.CollectGarbage`)
  (set `self.EscapeMenuRef` null)
  (`GameplayStatics.SetGlobalTimeDilation` 1.0)
  (`self.EnableInput` (`Controller.K2_GetPawn` _returnvalue) _returnvalue))

(event `SetupCurrentLevelWidget`
  (bind _returnvalue (`|CreateWidget` "/Game/Blueprints/Widgets/W_CurrentLevel.W_CurrentLevel_C" (`self.GetOwningPlayerController`)))
  (`UserWidget.AddToViewport` _returnvalue -40))

(event `SetupAndroid`
  (bind _returnvalue (`/Game/Blueprints/FunctionLibaries/BP_MobileFunctionLibrary.IsAndroid`))
  (if _returnvalue
    (bind _returnvalue_2 (`|CreateWidget` "/Game/Blueprints/Widgets/Mobile/W_Mobile_TouchButtons.W_Mobile_TouchButtons_C" (`self.GetOwningPlayerController`)))
    (`UserWidget.AddToPlayerScreen` _returnvalue_2 10)))

(fn `CanShowEscapeMenu`
  (returns (ReturnValue :type Boolean))
  (return (and (not (`KismetSystemLibrary.IsValid` (`self.InteractRef`))) (not (`KismetSystemLibrary.IsValid` (`self.EscapeMenuRef`))))))

(fn `UserConstructionScript`)