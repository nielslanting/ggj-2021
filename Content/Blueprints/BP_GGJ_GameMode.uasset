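; Game mode for a game jam level that sets up its goals, required score, player starting items and level-unlock save.
; On BeginPlay it loads or creates the save, unlocks the current map, feeds data-table-built goals to a GameState goal component and fills the pawn's inventory.
; GameState score component events freeze time and show complete or failed HUD widgets, with completion saving the next map's unlock.
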(event `self.ReceiveBeginPlay`
  (`self.SetupSaveGame`)
  (`self.SetupGoals`)
  (`self.SetupScoreComponentBinding`)
  (`self.SetupStartItems`))

(event `SetupGoals`
  (bind _returnvalue (`GameplayStatics.GetGameState`))
  (bind _returnvalue_2 (`self.GetComponentByClass` _returnvalue "/Game/Blueprints/GameStateComponents/BP_GameState_Goal_Component.BP_GameState_Goal_Component_C"))
  (for _array_element (`self.LevelGoals`)
    (bind _returnvalue_3 (`self.Create Goal` (`.Timer_7_2502603E494265938ABAEDBFEA7D1DC0` (break `/Game/Blueprints/BPS_Level_Goal` _array_element)) (break `/Game/Blueprints/BPS_Level_Goal` _array_element)))
    (`/Engine/EditorBlueprintResources/StandardMacros.IsValid` _returnvalue
      (:`Is Valid`
        (`/Engine/EditorBlueprintResources/StandardMacros.IsValid` _returnvalue_2
          (:`Is Valid`
            (`/Game/Blueprints/GameStateComponents/BP_GameState_Goal_Component.AddGoal` _returnvalue_2 _returnvalue_3)))))))

(event `SetupScoreComponentBinding`
  (bind _returnvalue (`GameplayStatics.GetGameState`))
  (bind _returnvalue_2 (`self.GetComponentByClass` _returnvalue "/Game/Blueprints/GameStateComponents/BP_GameState_Score_Component.BP_GameState_Score_Component_C"))
  (`/Engine/EditorBlueprintResources/StandardMacros.IsValid` _returnvalue
    (:`Is Valid`
      (`/Engine/EditorBlueprintResources/StandardMacros.IsValid` _returnvalue_2
        (:`Is Valid`
          (`/Game/Blueprints/GameStateComponents/BP_GameState_Score_Component.SetRequiredScore` _returnvalue_2 (`self.RequiredForNextLevel`))
          (add `/Game/Blueprints/GameStateComponents/BP_GameState_Score_Component.OnRequiredScoreReached` _returnvalue_2 (`|CreateDelegate` :!event `HandleOnRequiredScoreReached`))
          (add `/Game/Blueprints/GameStateComponents/BP_GameState_Score_Component.OnFailed` _returnvalue_2 (`|CreateDelegate` :!event `HandleFailed`)))))))

(event `HandleOnRequiredScoreReached`
  (`GameplayStatics.SetGlobalTimeDilation` 0.0)
  (bind _asbpi_hud_show_level_complete_widget (cast `/Game/Blueprints/Interfaces/BPI_HUD_ShowLevelCompleteWidget` (`PlayerController.GetHUD` (`GameplayStatics.GetPlayerController` 0))))
  (bind _returnvalue (`GameplayStatics.GetCurrentLevelName` true))
  (`/Game/Blueprints/Interfaces/BPI_HUD_ShowLevelCompleteWidget.ShowLevelCompleteWidget` _asbpi_hud_show_level_complete_widget _returnvalue "00:00" (`self.NextLevel`))
  (if (!= (`self.NextLevel`) "Finish")
    (`KismetArrayLibrary.Array_AddUnique` (`/Game/Blueprints/BP_GGJ_SaveGame.UnlockedMaps` (`self.SaveGameRef`)) (`self.NextLevel`))
    (`GameplayStatics.SaveGameToSlot` (`self.SaveGameRef`) "SaveSlot")))

(event `HandleFailed`
  (`GameplayStatics.SetGlobalTimeDilation` 0.0)
  (bind _asbpi_hud_show_level_complete_widget (cast `/Game/Blueprints/Interfaces/BPI_HUD_ShowLevelCompleteWidget` (`PlayerController.GetHUD` (`GameplayStatics.GetPlayerController` 0))))
  (`/Game/Blueprints/Interfaces/BPI_HUD_ShowLevelCompleteWidget.ShowLevelFailedWidget` _asbpi_hud_show_level_complete_widget))

(event `SetupStartItems`
  (for _array_element (`self.StartItems`)
    (bind _returnvalue (`|GetDataTableRow` (break `DataTableRowHandle` _array_element) (`.RowName` (break `DataTableRowHandle` _array_element)))
      (:`then`
        (`/Game/Blueprints/ActorComponents/BP_Inventory_ActorComponent.AddItem` (`self.GetComponentByClass` (`Controller.K2_GetPawn` (`GameplayStatics.GetPlayerController` 0)) "/Game/Blueprints/ActorComponents/BP_Inventory_ActorComponent.BP_Inventory_ActorComponent_C") _returnvalue)))))

(event `SetupSaveGame`
  (bind _returnvalue (`GameplayStatics.LoadGameFromSlot` "SaveSlot"))
  (bind _asbp_ggj_save_game (cast `/Game/Blueprints/BP_GGJ_SaveGame` _returnvalue)
    (:`then`
      (set `self.SaveGameRef` _asbp_ggj_save_game))
    (:`CastFailed`
      (bind _returnvalue_2 (`GameplayStatics.CreateSaveGameObject` "/Game/Blueprints/BP_GGJ_SaveGame.BP_GGJ_SaveGame_C"))
      (set `self.SaveGameRef` _returnvalue_2)))
  (bind _returnvalue_3 (`GameplayStatics.GetCurrentLevelName` true))
  (`KismetArrayLibrary.Array_AddUnique` (`/Game/Blueprints/BP_GGJ_SaveGame.UnlockedMaps` (`self.SaveGameRef`)) (`KismetStringLibrary.Conv_StringToName` _returnvalue_3))
  (`GameplayStatics.SaveGameToSlot` (`self.SaveGameRef`) "SaveSlot"))

(fn `Create Goal`
  (params (Timer :type Integer) (Rows :type "Array of DataTableRowHandle Structure"))
  (returns (ReturnValue :type "/Game/Blueprints/GameStateComponents/BPS_Goal Structure"))
  (locals (Items :type "Array of /Game/Data/BPS_Item Structure"))
  (for _array_element Rows
    (bind _returnvalue (`|GetDataTableRow` (break `DataTableRowHandle` _array_element) (`.RowName` (break `DataTableRowHandle` _array_element)))
      (:`then`
        (`KismetArrayLibrary.Array_Add` (`local.Items`) _returnvalue))))
  (return (make `/Game/Blueprints/GameStateComponents/BPS_Goal` (`local.Items`) (`local.Timer`))))

(fn `UserConstructionScript`)