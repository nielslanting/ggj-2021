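; Inventory actor component that holds a list of items up to a MaxItems capacity.
; AddItem appends only while space remains, and items can be removed by index, which returns the removed item, or as a list.
; ContainsItems checks a list of items by matching their names rather than the items themselves.
; Additions and removals fire an items-changed notification, once per entry for list removal.
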(event `self.ReceiveBeginPlay`)

(fn `AddItem`
  (params (Item :type "/Game/Data/BPS_Item Structure"))
  (bind _returnvalue (`self.CanAddItem`))
  (if _returnvalue
    (`KismetArrayLibrary.Array_Add` (`self.Items`) Item)
    (`self.OnItemsChanged`)))

(fn `CanAddItem`
  (returns (ReturnValue :type Boolean))
  (return (< (`KismetArrayLibrary.Array_Length` (`self.Items`)) (`self.MaxItems`))))

(fn `ContainsItems`
  (params (Items :type "Array of /Game/Data/BPS_Item Structure"))
  (returns (ReturnValue :type Boolean))
  (locals (LocalItems :type "Array of /Game/Data/BPS_Item Structure") (LocalItemsNames :type "Array of Text"))
  (for _array_element (`self.Items`)
    (`KismetArrayLibrary.Array_Add` (`local.LocalItemsNames`) (`.Name_6_CF25B77440ADBA1D3BC2D1BF2D8CEB1A` (break `/Game/Data/BPS_Item` _array_element))))
  (for (_array_element_2 _array_index) Items
    (if (not (`KismetArrayLibrary.Array_Contains` (`local.LocalItemsNames`) (`.Name_6_CF25B77440ADBA1D3BC2D1BF2D8CEB1A` (break `/Game/Data/BPS_Item` _array_element_2))))
      (return false)
      (else
        (`KismetArrayLibrary.Array_Remove` (`local.LocalItems`) _array_index))))
  (return true))

(fn `GetItems`
  (returns (ReturnValue :type "Array of /Game/Data/BPS_Item Structure"))
  (return (`self.Items`)))

(fn `RemoveItemByIndex`
  (params (Index :type Integer))
  (returns (ReturnValue :type "/Game/Data/BPS_Item Structure"))
  (locals (Result :type "/Game/Data/BPS_Item Structure"))
  (set `local.Result` (`|GetArrayItem` (`self.Items`) Index))
  (`KismetArrayLibrary.Array_Remove` (`self.Items`) Index)
  (`self.OnItemsChanged`)
  (return (`local.Result`)))

(fn `RemoveItems`
  (params (Items :type "Array of /Game/Data/BPS_Item Structure"))
  (for _array_element Items
    (`KismetArrayLibrary.Array_RemoveItem` (`self.Items`) _array_element)
    (`self.OnItemsChanged`)))