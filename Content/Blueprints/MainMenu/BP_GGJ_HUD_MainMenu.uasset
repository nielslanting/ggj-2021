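; Main menu HUD that creates the menu widget on BeginPlay and, on Android, adds a touch-button overlay at a higher Z-order.
; SetupCreditsWidget, not called within this graph, opens a single credits widget and sets Game and UI input mode focused on it.
; The widget's OnClose event removes it, clears the reference and triggers garbage collection.
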(event `self.ReceiveBeginPlay`
  (`self.SetupMainMenu`)
  (`self.SetupAndroid`))

(event `SetupCreditsWidget`
  (`/Engine/EditorBlueprintResources/StandardMacros.IsValid` (`self.CreditsRef`)
    (:`Is Not Valid`
      (bind _returnvalue (`|CreateWidget` "/Game/Blueprints/MainMenu/Widgets/W_Credits.W_Credits_C" (`self.GetOwningPlayerController`)))
      (bind _output_get (set `self.CreditsRef` _returnvalue))
      (add `/Game/Blueprints/MainMenu/Widgets/W_Credits.OnClose` _output_get (delegate `OnClose_Event_0`))
      (`UserWidget.AddToViewport` _output_get 0)
      (`WidgetBlueprintLibrary.SetInputMode_GameAndUIEx` (`self.GetOwningPlayerController`) _output_get))))

(event `OnClose_Event_0`
  (`Widget.RemoveFromParent` (`self.CreditsRef`))
  (set `self.CreditsRef` null)
  (`KismetSystemLibrary.CollectGarbage`))

(event `SetupAndroid`
  (bind _returnvalue (`/Game/Blueprints/FunctionLibaries/BP_MobileFunctionLibrary.IsAndroid`))
  (if _returnvalue
    (bind _returnvalue_2 (`|CreateWidget` "/Game/Blueprints/Widgets/Mobile/W_Mobile_TouchButtons.W_Mobile_TouchButtons_C" (`self.GetOwningPlayerController`)))
    (`UserWidget.AddToViewport` _returnvalue_2 10)))

(event `SetupMainMenu`
  (bind _returnvalue (`|CreateWidget` "/Game/Blueprints/MainMenu/Widgets/W_MainMenu.W_MainMenu_C" (`self.GetOwningPlayerController`)))
  (`UserWidget.AddToViewport` _returnvalue 0))

(fn `UserConstructionScript`)