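; Game state component that tracks a score, a required score and a failure count.
; Increasing the score fires an increase event, plus a target-reached event when it exactly equals the required score.
; Recording a failure increments the failure count and fires the failed event while score plus failures is at or below the required score.
; Changing the required score also broadcasts an update, and getters expose both score values.
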(fn `GetRequiredScore`
  (returns (ReturnValue :type Integer))
  (return (`self.RequiredScore`)))

(fn `GetScore`
  (returns (ReturnValue :type Integer))
  (return (`self.Score`)))

(fn `IncreaseFailed`
  (set `self.Failed` (+ (`self.Failed`) 1))
  (if (>= (`self.RequiredScore`) (+ (`self.Score`) (`self.Failed`)))
    (`self.OnFailed`)))

(fn `IncreaseScore`
  (set `self.Score` (+ (`self.Score`) 1))
  (`self.OnScoreIncreased`)
  (if (== (`self.Score`) (`self.RequiredScore`))
    (`self.OnRequiredScoreReached`)))

(fn `SetRequiredScore`
  (params (Input :type Integer))
  (set `self.RequiredScore` Input)
  (`self.OnRequiredScoreUpdated`))