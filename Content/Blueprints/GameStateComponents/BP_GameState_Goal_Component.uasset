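; Game state component that runs a sequential list of timed goals, each holding items and a time limit.
; Setting or adding goals starts the first countdown once, storing a UTC end time alongside a named timer.
; Finishing a goal clears the timer and fires a finished event, while expiry fires a failed event.
; Both paths advance the index and broadcast a goal change, which also fires when the list runs out.
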(event `self.ReceiveBeginPlay`)

(fn `AddGoal`
  (params (Input :type "/Game/Blueprints/GameStateComponents/BPS_Goal Structure"))
  (`KismetArrayLibrary.Array_Add` (`self.Goals`) (make `/Game/Blueprints/GameStateComponents/BPS_Goal` Input_Items_7_738242704F3DF8F655EBE297948F0B21 Input_Timer_5_2C56B21C491896BBBAF9C6A7B0A19284))
  (`self.CheckCanStart`))

(fn `CheckCanStart`
  (if (not (`self.HasStartedTimer`))
    (bind (_returnvalue _isvalid) (`self.GetCurrentGoal`))
    (if _isvalid
      (bind (_items _timer) (break `/Game/Blueprints/GameStateComponents/BPS_Goal` _returnvalue))
      (set `self.EndsAt` (+ (`KismetMathLibrary.UtcNow`) (`KismetMathLibrary.MakeTimespan` 0 0 0 _timer)))
      (`KismetSystemLibrary.K2_SetTimer` null "FailedRound" (`KismetMathLibrary.Conv_IntToDouble` _timer))
      (set `self.HasStartedTimer` true)
      (`self.GetCurrentGoal`)
      (`self.OnGoalChanged`))))

(fn `FailedRound`
  (`self.OnGoalFailed`)
  (`self.GoToNextGoal`))

(fn `FinishCurrentGoal`
  (`KismetSystemLibrary.K2_ClearTimer` null "FailedRound")
  (bind (_returnvalue _isvalid) (`self.GetCurrentGoal`))
  (if _isvalid
    (`self.OnGoalFinished` _returnvalue)
    (`self.GoToNextGoal`)))

(fn `GetCurrentGoal`
  (returns (ReturnValue :type "/Game/Blueprints/GameStateComponents/BPS_Goal Structure") (IsValid :type Boolean) (EndTime :type "DateTime Structure"))
  (if (not (> (`self.CurrentGoalIndex`) (- (`KismetArrayLibrary.Array_Length` (`self.Goals`)) 1)))
    (return (`|GetArrayItem` (`self.Goals`) (`self.CurrentGoalIndex`)) true (`self.EndsAt`))
    (else
      (return (struct) false))))

(fn `GetGoals`
  (returns (ReturnValue :type "Array of /Game/Blueprints/GameStateComponents/BPS_Goal Structure"))
  (return (`self.Goals`)))

(fn `GoToNextGoal`
  (set `self.CurrentGoalIndex` (+ (`self.CurrentGoalIndex`) 1))
  (bind (_returnvalue _isvalid) (`self.GetCurrentGoal`))
  (if _isvalid
    (bind (_items _timer) (break `/Game/Blueprints/GameStateComponents/BPS_Goal` _returnvalue))
    (`KismetSystemLibrary.K2_SetTimer` null "FailedRound" (`KismetMathLibrary.Conv_IntToDouble` _timer))
    (set `self.EndsAt` (+ (`KismetMathLibrary.UtcNow`) (`KismetMathLibrary.MakeTimespan` 0 0 0 _timer)))
    (`self.OnGoalChanged`)
    (else
      (`self.OnGoalChanged`))))

(fn `SetGoals`
  (params (Input :type "Array of /Game/Blueprints/GameStateComponents/BPS_Goal Structure"))
  (set `self.Goals` Input)
  (`self.CheckCanStart`))